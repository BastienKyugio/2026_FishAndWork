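; BP_RoomManager watches a room and penalizes the player for infractions found when it is scanned.
; Box overlaps track files, keys and top-sensitivity files on the floor, set player grounding, cache the manager AI, and release held movable objects on player exit.
; RoomIsScanned checks those states plus examining, key possession and overdue tasks.
; Each infraction adds suspicion and cycle stats to FishGameMode and angers the manager.
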(event OnComponentBeginOverlap(Box)
  (params (OverlappedComponent :type Primitive%20Component%20Object%20Reference) (OtherActor :type Actor%20Object%20Reference) (OtherComp :type Primitive%20Component%20Object%20Reference) (OtherBodyIndex :type Integer) (bFromSweep :type Boolean) (SweepResult :type Hit%20Result%20Structure%20%28by%20ref%29))
  (Utilities|FlowControl|Sequence
    (:then_0
      (bind _asbp_first_person_character (Utilities|Casting|CastToBP_FirstPersonCharacter OtherActor))
      (Variables|/Game/Player/BP_FirstPersonCharacter.BP_FirstPersonCharacter_C|SetIsGrounded _asbp_first_person_character true))
    (:then_1
      (if (Actor|ActorHasTag OtherActor "File")
        (bind _result (Math|Integer|IncrementInt (Variables|Default|GetFilesOnFloor))
          (:%20%20
            (Development|PrintString "(Room Manager) Objets au sol : ")
            (Development|PrintString (Utilities|String|ToString(Integer) _result))))))
    (:then_2
      (if (Actor|ActorHasTag OtherActor "Key")
        (Variables|Default|SetKeyOnFloor true)))
    (:then_3
      (bind _asbp_file (Utilities|Casting|CastToBP_FIle OtherActor))
      (if (== (Variables|/Game/Blueprint/BP_Data/BP_DA_Files.BP_DA_Files_C|GetLevelOfSensitivity (Variables|/Game/Blueprint/BP_FIle.BP_FIle_C|GetFileData _asbp_file)) 4)
        (Variables|Default|SetLevelSecretOnFloor true)))
    (:then_4
      (bind _asbp_manager_ai (Utilities|Casting|CastToBP_ManagerAi OtherActor))
      (Variables|Default|SetManagerAi _asbp_manager_ai))))

(event OnComponentEndOverlap(Box)
  (params (OverlappedComponent :type Primitive%20Component%20Object%20Reference) (OtherActor :type Actor%20Object%20Reference) (OtherComp :type Primitive%20Component%20Object%20Reference) (OtherBodyIndex :type Integer))
  (bind _ascharacter_controller (CallFunction|GetPlayerController))
  (Utilities|FlowControl|Sequence
    (:then_0
      (if (Actor|ActorHasTag OtherActor "File")
        (bind _result (Math|Integer|DecrementInt (Variables|Default|GetFilesOnFloor))
          (:%20%20
            (Development|PrintString "(Room Manager) Objets au sol : ")
            (Development|PrintString (Utilities|String|ToString(Integer) _result))))))
    (:then_1
      (bind _asbp_first_person_character (Utilities|Casting|CastToBP_FirstPersonCharacter OtherActor))
      (Variables|/Game/Player/BP_FirstPersonCharacter.BP_FirstPersonCharacter_C|SetIsGrounded _asbp_first_person_character false)
      (Utilities|IsValid _ascharacter_controller
        (:Is%20Valid
          (if (Variables|/Game/Player/BP_FirstPersonController.BP_FirstPersonController_C|GetIsHoldingMovableObject _ascharacter_controller)
            (Default|ReleaseNonPickableItem (CallFunction|GetPlayerController))))
        (:Is%20Not%20Valid
          (Development|PrintString "(Room Manager) Controller not valid "))))
    (:then_2
      (if (Actor|ActorHasTag OtherActor "Key")
        (Variables|Default|SetKeyOnFloor false)))
    (:then_3
      (bind _asbp_file (Utilities|Casting|CastToBP_FIle OtherActor))
      (if (== (Variables|/Game/Blueprint/BP_Data/BP_DA_Files.BP_DA_Files_C|GetLevelOfSensitivity (Variables|/Game/Blueprint/BP_FIle.BP_FIle_C|GetFileData _asbp_file)) 4)
        (Variables|Default|SetLevelSecretOnFloor false)))))

(event Custom|RoomIsScanned
  (bind _as_fish_game_mode (Variables|Default|GetAs%20Fish%20Game%20Mode))
  (bind _as_fish_game_mode_2 (Variables|Default|GetAs%20Fish%20Game%20Mode))
  (bind _as_fish_game_mode_3 (Variables|Default|GetAs%20Fish%20Game%20Mode))
  (bind _as_fish_game_mode_4 (Variables|Default|GetAs%20Fish%20Game%20Mode))
  (bind _as_fish_game_mode_5 (Variables|Default|GetAs%20Fish%20Game%20Mode))
  (bind _as_fish_game_mode_6 (Variables|Default|GetAs%20Fish%20Game%20Mode))
  (bind _cyclestats (Variables|/Game/Player/FishGameMode.FishGameMode_C|GetCycleStats _as_fish_game_mode))
  (bind _cyclestats_2 (Variables|/Game/Player/FishGameMode.FishGameMode_C|GetCycleStats _as_fish_game_mode_2))
  (bind _cyclestats_3 (Variables|/Game/Player/FishGameMode.FishGameMode_C|GetCycleStats _as_fish_game_mode_3))
  (bind _cyclestats_4 (Variables|/Game/Player/FishGameMode.FishGameMode_C|GetCycleStats _as_fish_game_mode_5))
  (bind _cyclestats_5 (Variables|/Game/Player/FishGameMode.FishGameMode_C|GetCycleStats _as_fish_game_mode_4))
  (bind _cyclestats_6 (Variables|/Game/Player/FishGameMode.FishGameMode_C|GetCycleStats _as_fish_game_mode_6))
  (Utilities|FlowControl|Sequence
    (:then_0
      (if (> (Variables|Default|GetFilesOnFloor) 0)
        (Development|PrintString "Manager pas content" true true "(R=1.000000,G=0.000000,B=0.000000,A=1.000000)")
        (Default|AddSuspicion (Variables|Default|GetAs%20Fish%20Game%20Mode) (Math|Conversions|ToFloat(Integer) (* (Variables|Default|GetFilesOnFloor) 10)))
        (Utilities|Struct|SetmembersinS_CycleStats _cyclestats_6 (+ (.Susp_Minor_FilesOnFloor (Utilities|Struct|BreakS_CycleStats _cyclestats_6)) 1))
        (Development|PrintString "files on floor")
        (bind _output_get (Variables|/Game/Blueprint/AI/BP_ManagerAi.BP_ManagerAi_C|SetAngry (Variables|Default|GetManagerAi) true :!label _label))
        (Development|PrintString (Utilities|String|ToString(Boolean) _output_get) true true "(R=0.056710,G=1.000000,B=0.000000,A=1.000000)")
        (else
          (Development|PrintString "Manager content"))))
    (:then_1
      (if (Variables|/Game/Player/BP_FirstPersonController.BP_FirstPersonController_C|GetIsExamining (CallFunction|GetPlayerController))
        (Default|AddSuspicion _as_fish_game_mode_4 3e+01)
        (Utilities|Struct|SetmembersinS_CycleStats _cyclestats_5 (+ (.Susp_Serious_CaughtExamining (Utilities|Struct|BreakS_CycleStats _cyclestats_5)) 1))
        (Development|PrintString "caught examining")
        (goto _label)))
    (:then_2
      (if (Variables|Default|GetKeyOnFloor)
        (Default|AddSuspicion _as_fish_game_mode_2 1e+01)
        (Utilities|Struct|SetmembersinS_CycleStats _cyclestats_2 (+ (.Susp_Minor_LockerKeyOnFloor (Utilities|Struct|BreakS_CycleStats _cyclestats_2)) 1))
        (Development|PrintString "key on floor")
        (goto _label)))
    (:then_3
      (if (Variables|Default|GetLevelSecretOnFloor)
        (Default|AddSuspicion _as_fish_game_mode_3 5e+01)
        (Utilities|Struct|SetmembersinS_CycleStats _cyclestats_3 (+ (.Susp_Conspir_FoundLvlSecret (Utilities|Struct|BreakS_CycleStats _cyclestats_3)) 1))
        (Development|PrintString "scrt lvl")
        (goto _label)))
    (:then_4
      (if (Variables|/Game/Player/BP_FirstPersonController.BP_FirstPersonController_C|GetHasKey (CallFunction|GetPlayerController))
        (Default|AddSuspicion _as_fish_game_mode_5 5e+01)
        (Utilities|Struct|SetmembersinS_CycleStats _cyclestats_4 (+ (.Susp_Conspir_CaughtHavingLockerKey (Utilities|Struct|BreakS_CycleStats _cyclestats_4)) 1))
        (Development|PrintString "key on hand")
        (goto _label)))
    (:then_5
      (if (Variables|/Game/Player/FishGameMode.FishGameMode_C|GetTimeLimitForTasks (Variables|Default|GetAs%20Fish%20Game%20Mode))
        (if (Variables|/Game/Player/FishGameMode.FishGameMode_C|GetTasksAreCompleted (Variables|Default|GetAs%20Fish%20Game%20Mode))
          (Development|PrintString "TaskAreCompleted")
          (else
            (Default|AddSuspicion _as_fish_game_mode 3e+01)
            (Utilities|Struct|SetmembersinS_CycleStats _cyclestats (+ (.Susp_Serious_TaskNoCompleted (Utilities|Struct|BreakS_CycleStats _cyclestats)) 1))
            (Development|PrintString "TaskNotCompleted")
            (goto _label)))))))

(event EventBeginPlay
  (bind _asfish_game_mode (Utilities|Casting|CastToFishGameMode (Game|GetGameMode)))
  (Variables|Default|SetAs%20Fish%20Game%20Mode _asfish_game_mode))

(fn ConstructionScript)