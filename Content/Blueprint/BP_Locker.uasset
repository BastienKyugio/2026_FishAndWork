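; BP_Locker is an interactable locker whose door opens only if the player controller holds a key.
; ChangeStateDoor toggles the door, playing an open or close sound while a Timeline drives the door mesh's yaw through 90 degrees, reversed to close.
; Without the key, it prints a message, plays a fail sound and briefly flashes the HUD's error crosshair with shake animations.
; GetItemPickable reports a fixed item enum value.
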(event Custom|ChangeStateDoor
  (bind _ascharacter_controller (CallFunction|GetPlayerController))
  (bind _returnvalue (Transformation|GetActorLocation))
  (bind _ascharacter_controller_2 (CallFunction|GetPlayerController))
  (bind _hud (Variables|/Game/Player/BP_FirstPersonController.BP_FirstPersonController_C|GetHUD _ascharacter_controller_2))
  (bind _hud_2 (Variables|/Game/Player/BP_FirstPersonController.BP_FirstPersonController_C|GetHUD _ascharacter_controller))
  (if (Variables|Default|GetIsDoorOpen)
    (Audio|PlaySoundatLocation "/Game/Sound_Design/SFX/SD_ClosingLocker.SD_ClosingLocker" _returnvalue "0, 0, 0" 1.0 1.0 0.0 "/Game/Sound_Design/SA_Monospacialisation.SA_Monospacialisation" 0 0 0)
    (Variables|Default|SetIsDoorOpen false)
    (bind _newtrack_0 (Timeline|Timeline Reverse)
      (:Update
        (Transformation|SetRelativeRotation (Variables|Default|GetGEO_Door_Locker) (Math|Rotator|MakeRotator 0.0 0.0 (* _newtrack_0 -9e+01)) false false)))
    (elif (Variables|/Game/Player/BP_FirstPersonController.BP_FirstPersonController_C|GetHasKey (CallFunction|GetPlayerController))
      (Audio|PlaySoundatLocation "/Game/Sound_Design/MSS_OpeningLocker.MSS_OpeningLocker" _returnvalue "0, 0, 0" 1.0 1.0 0.0 "/Game/Sound_Design/SA_Monospacialisation.SA_Monospacialisation" 0 0 0)
      (Variables|Default|SetIsDoorOpen true)
      (Timeline|Timeline Play)
      (else
        (Development|PrintString "N'a  pas les clé")
        (Audio|PlaySound2D "/Game/Sound_Design/MSS_FailInteraction.MSS_FailInteraction" 1.0 1.0 0.0 0 0)
        (Widget|SetVisibility (Variables|/Game/UI/WBP_HUD.WBP_HUD_C|GetCrossHairObjectTargeted _hud_2) "Hidden")
        (Widget|SetVisibility (Variables|/Game/UI/WBP_HUD.WBP_HUD_C|GetCrossHairObjectError _hud_2) "Visible")
        (UserInterface|Animation|PlayAnimation _hud_2 (Variables|/Game/UI/WBP_HUD.WBP_HUD_C|GetError _hud_2) 0.0 1 "Forward" 1.0 false)
        (UserInterface|Animation|PlayAnimation _hud_2 (Variables|/Game/UI/WBP_HUD.WBP_HUD_C|GetShakeCrossHair _hud_2) 0.0 1 "Forward" 1.0 false)
        (Utilities|FlowControl|Delay 0.2)
        (Widget|SetVisibility (Variables|/Game/UI/WBP_HUD.WBP_HUD_C|GetCrossHairObjectTargeted _hud) "Visible")
        (Widget|SetVisibility (Variables|/Game/UI/WBP_HUD.WBP_HUD_C|GetCrossHairObjectError _hud) "Hidden")))))

(fn ConstructionScript)

(fn GetItemPickable
  (return "NewEnumerator2"))