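; BP_GEODoor is a door actor that swings open and closed by rotating its GEODoor component around world yaw.
; OpenDoor and CloseDoor events play the Opening and Closing timelines from the start.
; Each timeline update subtracts or adds its track value to the current yaw while zeroing pitch and roll, so rotation accumulates per tick rather than interpolating between fixed angles.
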(event Custom|CloseDoor
  (bind _newtrack_0 (Timeline|Closing PlayFromStart)
    (:Update
      (Transformation|SetWorldRotation (Variables|Default|GetGEO_Door) (Math|Rotator|MakeRotator 0.0 0.0 (+ (.yaw (Transformation|GetWorldRotation (Variables|Default|GetGEO_Door))) _newtrack_0)) false false))))

(event Custom|OpenDoor
  (bind _newtrack_0 (Timeline|opening PlayFromStart)
    (:Update
      (Transformation|SetWorldRotation (Variables|Default|GetGEO_Door) (Math|Rotator|MakeRotator 0.0 0.0 (- (.yaw (Transformation|GetWorldRotation (Variables|Default|GetGEO_Door))) _newtrack_0)) false false))))

(fn ConstructionScript)