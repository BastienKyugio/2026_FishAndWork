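; BP_Interactable_Base is a base interactable item that toggles its skeletal mesh's physics and collision as it is interacted with and dropped.
; Construction leaves the mesh static with query and physics collision, and OnInteract turns off both simulation and collision.
; OnDrop re-enables simulation but sets collision to query-only rather than restoring physics collision.
; GetItemPickable reports a fixed enum value for the item's pickable type.
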(event EventOnInteract
  (bind _skeletalmesh (Variables|Default|GetSkeletalMesh))
  (Physics|SetSimulatePhysics _skeletalmesh false)
  (Collision|SetCollisionEnabled _skeletalmesh "NoCollision"))

(event EventOnDrop
  (bind _skeletalmesh (Variables|Default|GetSkeletalMesh))
  (Collision|SetCollisionEnabled _skeletalmesh "QueryOnly")
  (Physics|SetSimulatePhysics _skeletalmesh true))

(fn ConstructionScript
  (bind _skeletalmesh (Variables|Default|GetSkeletalMesh))
  (Collision|SetCollisionEnabled _skeletalmesh "QueryAndPhysics")
  (Physics|SetSimulatePhysics _skeletalmesh false))

(fn GetItemPickable
  (return "NewEnumerator1"))