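; BP_CartDay1 is an interactable cart that holds the starting set of file objects, apparently for the game's first day.
; On BeginPlay it spawns a BP_FIle for each initial data entry, disables its physics, tags it as cart content, snaps it to one of five slots and records it in Files.
; The SDCart component plays on each spawn.
; OnInteract is unfinished, looping over slots without acting when the player holds an object.
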(event EventBeginPlay
  (bind _output_get (Variables|Default|SetSlotsList (Utilities|Array|MakeArray (Variables|Default|GetSlot_01) (Variables|Default|GetSlot_02) (Variables|Default|GetSlot_03) (Variables|Default|GetSlot_04) (Variables|Default|GetSlot_05))))
  (Utilities|Array|Resize (Variables|Default|GetFiles) (Utilities|Array|Length _output_get))
  (for (_array_element _array_index) (Variables|Default|GetInitialFilesToSpawn)
    (bind _returnvalue (Game|SpawnActorfromClass "/Game/Blueprint/BP_FIle.BP_FIle_C" (Transformation|GetRelativeTransform (Utilities|Array|Get(acopy) (Variables|Default|GetSlotsList) _array_index)) "Undefined" "MultiplyWithRoot" 0 _array_element 0))
    (Physics|SetSimulatePhysics (Variables|/Game/Blueprint/BP_Interactable_Base.BP_Interactable_Base_C|GetSkeletalMesh _returnvalue) false)
    (Utilities|Array|AddUnique (Variables|/Script/Engine.Actor|GetTags _returnvalue) "Cart")
    (Transformation|AttachComponentToComponent _returnvalue (Utilities|Array|Get(acopy) (Variables|Default|GetSlotsList) _array_index) "None" "SnapToTarget" "SnapToTarget" "SnapToTarget" true)
    (Utilities|Array|SetArrayElem (Variables|Default|GetFiles) _array_index _returnvalue)
    (Audio|Components|Audio|Play (Variables|Default|GetSD_Cart) 5.5)))

(event EventOnInteract
  (Utilities|IsValid (Variables|/Game/Player/BP_FirstPersonController.BP_FirstPersonController_C|GetHeldObject (CallFunction|GetPlayerController))
    (:Is%20Valid
      (for _array_element (Variables|Default|GetSlotsList)
        _))))

(fn ConstructionScript)

(fn GetItemPickable
  (return "NewEnumerator2"))