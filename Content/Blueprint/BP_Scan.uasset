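; Scanner machine that takes a fully analysed BP_FIle held by the player, marks it scanned and records its data.
; OnScan drops the file and uses chained timelines to move it through entry and middle anchors before a timed scan.
; FinishScan adds the data to ScannedFilesList, ejects the file via the exit anchor with a physics impulse, and can trigger boss scan dialogue through FishGameMode.
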(event Custom|OnScan
  (bind _ascharacter_controller (CallFunction|GetPlayerController))
  (bind _anchor_entry (Variables|Default|GetAnchor_Entry))
  (bind _anchor_middle (Variables|Default|GetAnchor_Middle))
  (bind _heldobject (Variables|/Game/Player/BP_FirstPersonController.BP_FirstPersonController_C|GetHeldObject _ascharacter_controller))
  (if (not (Variables|Default|GetIsScanning))
    (bind _asbp_file (Utilities|Casting|CastToBP_FIle (Variables|/Game/Player/BP_FirstPersonController.BP_FirstPersonController_C|GetHeldObject (CallFunction|GetPlayerController))))
    (Utilities|IsValid _asbp_file
      (:Is%20Valid
        (Variables|Default|SetObjectOnScan _asbp_file)
        (if (>= (Variables|/Game/Blueprint/BP_FIle.BP_FIle_C|GetCurrentAnalysisProgress _asbp_file) 1.0)
          (Variables|/Game/Blueprint/BP_FIle.BP_FIle_C|SetCurrentIsScanned _asbp_file true)
          (Variables|Default|SetCurrentScanningFile (Variables|/Game/Blueprint/BP_FIle.BP_FIle_C|GetFileData _asbp_file))
          (Variables|/Game/Blueprint/BP_FIle.BP_FIle_C|SetOnScan _asbp_file true)
          (Utilities|IsValid _heldobject
            (:Is%20Valid
              (bind _asbp_file_2 (Utilities|Casting|CastToBP_FIle _heldobject))
              (Variables|Default|SetObjectOnScan _asbp_file_2)
              (Variables|Default|SetStartTransform (Transformation|GetWorldTransform (Variables|/Game/Player/BP_FirstPersonCharacter.BP_FirstPersonCharacter_C|GetHoldObject (CallFunction|GetPlayerCharacter))))
              (Default|DropPickableItem (CallFunction|GetPlayerController))
              (Physics|SetSimulatePhysics (Variables|/Game/Blueprint/BP_Interactable_Base.BP_Interactable_Base_C|GetStaticMesh _asbp_file_2) false)
              (bind _newtrack_0 (Timeline|Timeline Play)
                (:Update
                  (Transformation|SetActorTransform (Variables|Default|GetObjectOnScan) (Math|Transform|Lerp(Transform) (Variables|Default|GetStartTransform) (Transformation|GetWorldTransform _anchor_entry) _newtrack_0))
                  (Transformation|SetActorRotation (Variables|Default|GetObjectOnScan) (Variables|/Script/Engine.SceneComponent|GetRelativeRotation _anchor_entry)))
                (:Finished
                  (Audio|PlaySoundatLocation "/Game/Sound_Design/SFX/SD_Scan.SD_Scan" (Transformation|GetActorLocation) "0, 0, 0" 0.6 1.0 0.0 "/Game/Sound_Design/SA_Monospacialisation.SA_Monospacialisation" 0 0 0)
                  (Transformation|AttachComponentToComponent (Variables|Default|GetObjectOnScan) (Variables|Default|GetAnchor_Entry) "None" "SnapToTarget" "SnapToTarget" "SnapToTarget" true)
                  (Variables|Default|SetStartTransform (Transformation|GetWorldTransform (Variables|Default|GetAnchor_Entry)))
                  (Transformation|DetachFromActor (Variables|Default|GetObjectOnScan) "KeepWorld" "KeepWorld" "KeepWorld")
                  (bind _newtrack_0_2 (Timeline|Timeline_0 PlayFromStart)
                    (:Update
                      (Transformation|SetActorTransform (Variables|Default|GetObjectOnScan) (Math|Transform|Lerp(Transform) (Variables|Default|GetStartTransform) (Transformation|GetWorldTransform _anchor_middle) _newtrack_0_2))
                      (Transformation|SetActorRotation (Variables|Default|GetObjectOnScan) (Variables|/Script/Engine.SceneComponent|GetRelativeRotation _anchor_middle)))
                    (:Finished
                      (CallFunction|StartScan))))))))))))

(event Custom|ExpulseFile
  (bind _anchor_exit (Variables|Default|GetAnchor_Exit))
  (bind _returnvalue (Math|Vector|GetUpVector _anchor_exit))
  (Variables|Default|SetStartTransform (Transformation|GetWorldTransform (Variables|Default|GetAnchor_Middle)))
  (bind _newtrack_0 (Timeline|Timeline_1 PlayFromStart)
    (:Update
      (Transformation|SetActorTransform (Variables|Default|GetObjectOnScan) (Math|Transform|Lerp(Transform) (Variables|Default|GetStartTransform) (Transformation|GetWorldTransform (Variables|Default|GetAnchor_Exit)) _newtrack_0)))
    (:Finished
      (bind _asbp_file (Utilities|Casting|CastToBP_FIle (Variables|Default|GetObjectOnScan)))
      (Collision|SetCollisionEnabled (Variables|/Game/Blueprint/BP_Interactable_Base.BP_Interactable_Base_C|GetStaticMesh _asbp_file) "QueryAndPhysics")
      (Physics|SetSimulatePhysics (Variables|/Game/Blueprint/BP_Interactable_Base.BP_Interactable_Base_C|GetStaticMesh _asbp_file) true)
      (Physics|AddImpulse (Variables|/Game/Blueprint/BP_Interactable_Base.BP_Interactable_Base_C|GetStaticMesh _asbp_file) (Math|Vector|MakeVector (+ (.x _returnvalue) (Variables|Default|GetThrowForce)) (.y _returnvalue) (+ (.z _returnvalue) 3e+02)) "None" true))))

(event EventTick
  (params (DeltaSeconds :type Float%20%28single-precision%29)))

(fn ConstructionScript)

(fn StartScan
  (Variables|Default|SetIsScanning true)
  (Development|PrintString "(Scanner) Le scan de l'objet commence")
  (Utilities|Time|SetTimerbyFunctionName 0 "FinishScan" (Variables|Default|GetScanDuration)))

(fn FinishScan
  (Utilities|Array|Add (Variables|Default|GetScannedFilesList) (Variables|Default|GetCurrentScanningFile))
  (bind _asbp_file (Utilities|Casting|CastToBP_FIle (Variables|Default|GetObjectOnScan))
    (:then
      (Variables|/Game/Blueprint/BP_FIle.BP_FIle_C|SetOnScan _asbp_file false)
      (Variables|Default|SetCurrentScanningFile 0)
      (Variables|Default|SetIsScanning false)
      (Development|PrintString "(Scanner) Le scan de l'objet est fini")
      (CallFunction|ExpulseFile)
      (bind _asfish_game_mode (Utilities|Casting|CastToFishGameMode (Game|GetGameMode)))
      (if (and (not (Variables|/Game/UI/WBP_OnBoarding.WBP_OnBoarding_C|GetFirstBossScan (Variables|/Game/Player/FishGameMode.FishGameMode_C|GetDialogue _asfish_game_mode))) (Variables|/Game/UI/WBP_OnBoarding.WBP_OnBoarding_C|GetFirstBossInter (Variables|/Game/Player/FishGameMode.FishGameMode_C|GetDialogue _asfish_game_mode)))
        (Default|BossDialogueScan (Variables|/Game/Player/FishGameMode.FishGameMode_C|GetDialogue _asfish_game_mode)))
      (return))
    (:CastFailed
      (Development|PrintString "pas un file"))))

(fn GetItemPickable
  (return "NewEnumerator1"))