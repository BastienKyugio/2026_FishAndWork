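; BP_FIle is a pickable file item that the player takes from a shelf, with its mesh set from FileData at construction.
; On interact, it plays a grab sound, clears its slot in the parent BP_shelf's Files array and detaches.
; A timeline lerps it to the player's HoldObject before the PlayerController grabs it.
; It can be flagged as a task target with a material swap, and pickup clears that flag.
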(event Custom|SmoothPickup
  (if (Variables|Default|GetIsTaskTarget)
    (Variables|Default|SetIsTaskTarget false))
  (Variables|Default|SetStartTransform (Transformation|GetActorTransform))
  (bind _newtrack_0 (Timeline|LerpTimeline PlayFromStart)
    (:Update
      (Transformation|SetActorTransform (Math|Transform|Lerp(Transform) (Variables|Default|GetStartTransform) (Transformation|GetWorldTransform (Variables|/Game/Player/BP_FirstPersonCharacter.BP_FirstPersonCharacter_C|GetHoldObject (CallFunction|GetPlayerCharacter))) _newtrack_0)))
    (:Finished
      (Default|GrabPickableItem (CallFunction|GetPlayerController) self))))

(event Custom|ActivateTaskHighLight
  (Variables|Default|SetIsTaskTarget true)
  (Rendering|Material|SetMaterial (Variables|Default|GetStaticMesh) 0 "/DatasmithContent/Materials/AliasReference.AliasReference"))

(event EventBeginPlay
  (|CallParentFunction))

(event Collision|EventActorBeginOverlap
  (params (OtherActor :type Actor%20Object%20Reference))
  (|CallParentFunction OtherActor) ; This node is disabled and will not be called.\nDrag off pins to build functionality.
)

(event EventTick
  (params (DeltaSeconds :type Float%20%28single-precision%29))
  (|CallParentFunction DeltaSeconds) ; This node is disabled and will not be called.\nDrag off pins to build functionality.
)

(event EventOnInteract
  (|CallParentFunction)
  (bind _asbp_shelf (Utilities|Casting|CastToBP_shelf (Actor|GetAttachParentActor)))
  (Audio|PlaySound2D "/Game/Sound_Design/MSS_WaterGrab.MSS_WaterGrab" 1.5 1.0 0.0 0 0)
  (Utilities|Array|SetArrayElem (Variables|/Game/Blueprint/BP_shelf.BP_shelf_C|GetFiles _asbp_shelf) (Utilities|Array|FindItem (Variables|/Game/Blueprint/BP_shelf.BP_shelf_C|GetFiles _asbp_shelf) self) 0)
  (Transformation|DetachFromActor "KeepWorld" "KeepWorld" "KeepWorld")
  (CallFunction|SmoothPickup))

(event EventOnDrop
  (|CallParentFunction))

(event EventOnExamine)

(event EventOnPick)

(fn ConstructionScript
  (|CallParentFunction)
  (Utilities|IsValid (Variables|Default|GetFileData)
    (:Is%20Valid
      (Components|StaticMesh|SetStaticMesh (Variables|Default|GetStaticMesh) (Variables|/Game/Blueprint/BP_Data/BP_DA_Files.BP_DA_Files_C|GetDefaultMesh (Variables|Default|GetFileData))))))

(fn GetInspectableMesh
  (return 0 "0, 0, 0" 0))

(fn GetActorClass
  (return 0))

(fn GetItemPickable
  (return "NewEnumerator1"))