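; Manager AI that delivers a cart along a patrol route in the fish game.
; On BeginPlay it spawns a BP_Cart and attaches it to its anchor.
; MoveToNextPoint, not called within this graph, recursively chains AI moves through CartPatrolPoints.
; At the last point it pauses, detaches the cart, returns to the first point, then triggers FishGameMode's AI spawn check and file task before destroying itself.
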(event Custom|MoveToNextPoint
  (bind _cart_patrolpoints (Variables|Default|GetCart_PatrolPoints))
  (bind _currentpointindex (Variables|Default|GetCurrentPointIndex))
  (bind _as_fish_game_mode (Variables|Default|GetAs%20Fish%20Game%20Mode))
  (bind _output (Utilities|Array|Get(acopy) _cart_patrolpoints _currentpointindex))
  (Utilities|IsValid _output
    (:Is%20Valid
      (AI|AIMoveTo self (Transformation|GetActorLocation _output) 0 5e+01 false
        (:OnSuccess
          (Development|PrintString "(AI_Manager)  Le Manager a atteint un autre point")
          (if (== (Variables|Default|GetCurrentPointIndex) (Utilities|Array|LastIndex (Variables|Default|GetCart_PatrolPoints)))
            (Utilities|FlowControl|Delay 5.0)
            (Transformation|DetachFromActor (Variables|Default|GetCart) "KeepWorld" "KeepWorld" "KeepWorld")
            (AI|AIMoveTo self (Transformation|GetActorLocation (Utilities|Array|Get(acopy) (Variables|Default|GetCart_PatrolPoints))) 0 5e+01 false
              (:OnSuccess
                (Development|PrintString "Fin de pattern")
                (Default|CheckAISpawn _as_fish_game_mode 3)
                (Default|StartFileTask _as_fish_game_mode)
                (Actor|DestroyActor)))
            (else
              (Math|Integer|IncrementInt (Variables|Default|GetCurrentPointIndex)
                (:%20%20
                  (CallFunction|MovetoNextPoint))))))
        (:OnFail
          (Development|PrintString "(AI_Manager) Le Manager n'a pas atteint l'autre point"))))
    (:Is%20Not%20Valid
      (Development|PrintString (Utilities|String|ToString(Integer) (Utilities|Array|Length (Variables|Default|GetCart_PatrolPoints)))))))

(event EventBeginPlay
  (bind _asfish_game_mode (Utilities|Casting|CastToFishGameMode (Game|GetGameMode)))
  (Variables|Default|SetAs%20Fish%20Game%20Mode _asfish_game_mode)
  (bind _returnvalue (Game|SpawnActorfromClass "/Game/Blueprint/BP_Cart.BP_Cart_C" (Math|Transform|MakeTransform (Transformation|GetWorldLocation (Variables|Default|GetAnchorForCart)) "0, 0, 0" "1.000000,1.000000,1.000000") "Undefined" "MultiplyWithRoot" 0 0))
  (bind _output_get (Variables|Default|SetCart _returnvalue))
  (Transformation|AttachComponentToComponent _output_get (Variables|Default|GetAnchorForCart) "None" "SnapToTarget" "SnapToTarget" "SnapToTarget" true))

(fn ConstructionScript)