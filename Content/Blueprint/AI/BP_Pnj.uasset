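; Manager NPC that patrols a room through an indexed point list, searches it and reacts angrily if the room reports Caught.
; On spawn it scales walk speed by a game mode coefficient and, while the maze is unfinished, carries a key and gets target-locked by the player.
; A recursive AI MoveTo chain drives animation states and the door, then returns to the start, notifies FishGameMode and destroys itself.
; Overlapping BP_RoomManager resets Caught and triggers its scan.
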(event OnComponentBeginOverlap(CapsuleComponent)
  (params (OverlappedComponent :type Primitive%20Component%20Object%20Reference) (OtherActor :type Actor%20Object%20Reference) (OtherComp :type Primitive%20Component%20Object%20Reference) (OtherBodyIndex :type Integer) (bFromSweep :type Boolean) (SweepResult :type Hit%20Result%20Structure%20%28by%20ref%29))
  (bind _asbp_room_manager (Utilities|Casting|CastToBP_RoomManager OtherActor))
  (Variables|/Game/Blueprint/BP_RoomManager.BP_RoomManager_C|SetCaught _asbp_room_manager false)
  (bind _output_get (Variables|Default|SetAs%20BP%20Room%20Manager _asbp_room_manager))
  (Default|RoomIsScanned _output_get)
  (Development|PrintString "RoomIsScanned" true true "(R=1.000000,G=0.000000,B=0.000000,A=1.000000)"))

(event Custom|MoveToNextPoint
  (bind _manager_patrolpoints (Variables|Default|GetManager_PatrolPoints))
  (bind _currentpointindex (Variables|Default|GetCurrentPointIndex))
  (bind _as_bp_room_manager (Variables|Default|GetAs%20BP%20Room%20Manager))
  (bind _output (Utilities|Array|Get(acopy) _manager_patrolpoints _currentpointindex))
  (bind _caught (Variables|/Game/Blueprint/BP_RoomManager.BP_RoomManager_C|GetCaught _as_bp_room_manager))
  (Utilities|IsValid _output
    (:Is%20Valid
      (Default|SetWalk (Variables|Default|GetAs%20ABP%20Manager))
      (AI|AIMoveTo self (Transformation|GetActorLocation _output) 0 5e+01 false
        (:OnSuccess
          (Development|PrintString "(AI_Manager)  Le Manager a atteint un autre point")
          (if (== (Variables|Default|GetCurrentPointIndex) (Utilities|Array|LastIndex (Variables|Default|GetManager_PatrolPoints)))
            (Default|LockTarget (CallFunction|GetPlayerCharacter) self)
            (Default|SetSearch (Variables|Default|GetAs%20ABP%20Manager))
            (Utilities|FlowControl|Delay 3.2)
            (if _caught
              (Default|SetAngry (Variables|Default|GetAs%20ABP%20Manager))
              (Utilities|FlowControl|Delay 2.0)
              (else
                (Development|PrintString (Utilities|String|ToString(Boolean) _caught) true true "(R=0.000459,G=0.208333,B=0.031381,A=1.000000)")))
            (Default|SetWalk (Variables|Default|GetAs%20ABP%20Manager))
            (AI|AIMoveTo self (Transformation|GetActorLocation (Utilities|Array|Get(acopy) (Variables|Default|GetManager_PatrolPoints))) 0 5e+01 false
              (:then
                (Utilities|FlowControl|Delay 0.5)
                (Default|CloseDoor (Variables|Default|GetDoor)))
              (:OnSuccess
                (Development|PrintString "Fin de pattern")
                (Default|CheckAISpawn (Variables|Default|GetAs%20Fish%20Game%20Mode) 2)
                (Actor|DestroyActor)))
            (else
              (if (== (Variables|Default|GetCurrentPointIndex) 1)
                (Development|PrintString "Porte")
                (Default|OpenDoor (Variables|Default|GetDoor)))
              (if (== (Variables|Default|GetCurrentPointIndex) 3)
                (Development|PrintString "aaaaaaaaaaaaaaaaaaa" true true "(R=1.000000,G=0.869671,B=0.000000,A=1.000000)")
                (Default|SetUnderDoor (Variables|Default|GetAs%20ABP%20Manager))
                (Utilities|FlowControl|Delay 0.8))
              (Math|Integer|IncrementInt (Variables|Default|GetCurrentPointIndex)
                (:%20%20
                  (CallFunction|MovetoNextPoint))))))
        (:OnFail
          (Development|PrintString "(AI_Manager) Le Manager n'a pas atteint l'autre point"))))
    (:Is%20Not%20Valid
      (Development|PrintString (Utilities|String|ToString(Integer) (Utilities|Array|Length (Variables|Default|GetManager_PatrolPoints)))))))

(event EventBeginPlay
  (bind _charactermovement (Variables|Character|GetCharacterMovement))
  (bind _asabp_manager (Utilities|Casting|CastToABP_Manager (Components|SkeletalMesh|GetAnimInstance (Variables|Character|GetMesh))))
  (Variables|Default|SetAs%20ABP%20Manager _asabp_manager)
  (bind _asfish_game_mode (Utilities|Casting|CastToFishGameMode (Game|GetGameMode)))
  (bind _output_get (Variables|Default|SetAs%20Fish%20Game%20Mode _asfish_game_mode))
  (Variables|/Script/Engine.CharacterMovementComponent|SetMaxWalkSpeed _charactermovement (* (Variables|/Game/Player/FishGameMode.FishGameMode_C|GetCoef _output_get) (Variables|/Script/Engine.CharacterMovementComponent|GetMaxWalkSpeed _charactermovement)))
  (if (not (Variables|/Game/Player/BP_FirstPersonController.BP_FirstPersonController_C|GetMazeIsFinished (CallFunction|GetPlayerController)))
    (bind _returnvalue (Game|SpawnActorfromClass "/Game/Blueprint/BP_Key.BP_Key_C" (Math|Transform|MakeTransform (Transformation|GetWorldLocation (Variables|Default|GetAnchor_Key)) "0, 0, 0" "1.000000,1.000000,1.000000") "AlwaysSpawn" "MultiplyWithRoot" 0 0))
    (Physics|SetSimulatePhysics (Variables|/Game/Blueprint/BP_Interactable_Base.BP_Interactable_Base_C|GetSkeletalMesh _returnvalue) false)
    (Transformation|AttachComponentToComponent _returnvalue (Variables|Default|GetAnchor_Key) "None" "SnapToTarget" "SnapToTarget" "SnapToTarget" true)
    (Development|PrintString "cle a spawn" true true "(R=1.000000,G=0.666175,B=0.000000,A=1.000000)")
    (Utilities|FlowControl|Delay 3.0)
    (Default|LockTarget (CallFunction|GetPlayerCharacter) self)
    (else
      (Development|PrintString "Maze Fini" true true "(R=1.000000,G=0.747710,B=0.000000,A=1.000000)"))))

(fn ConstructionScript)