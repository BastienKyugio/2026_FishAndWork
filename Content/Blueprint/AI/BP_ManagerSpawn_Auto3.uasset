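; BP_ManagerSpawn_Auto3 is a spawner that creates manager and scientist AI characters at its own location.
; Two separate events spawn BP_ManagerAi or BP_ComputerScientist with no-collision-fail enabled.
; Each hands the new pawn the spawner's TargetPointsSpawner as patrol points, then calls MoveToNextPoint to start its patrol.
; The file contains no trigger for either event, so spawning depends on outside callers.
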(event Custom|SpawnScientistAI
  (bind _returnvalue (AI|SpawnAIFromClass "/Game/Blueprint/AI/BP_ComputerScientist.BP_ComputerScientist_C" 0 (Transformation|GetActorLocation) "0, 0, 0" true 0))
  (bind _asbp_computer_scientist (Utilities|Casting|CastToBP_ComputerScientist _returnvalue))
  (Variables|/Game/Blueprint/AI/BP_ComputerScientist.BP_ComputerScientist_C|SetPatrolPoints _asbp_computer_scientist (Variables|Default|GetTargetPointsSpawner))
  (Default|MovetoNextPoint _asbp_computer_scientist))

(event Custom|SpawnManagerAI
  (bind _returnvalue (AI|SpawnAIFromClass "/Game/Blueprint/AI/BP_ManagerAi.BP_ManagerAi_C" 0 (Transformation|GetActorLocation) "0, 0, 0" true 0))
  (bind _asbp_manager_ai (Utilities|Casting|CastToBP_ManagerAi _returnvalue))
  (Variables|/Game/Blueprint/AI/BP_ManagerAi.BP_ManagerAi_C|SetPatrolPoints _asbp_manager_ai (Variables|Default|GetTargetPointsSpawner))
  (Default|MovetoNextPoint _asbp_manager_ai))

(fn ConstructionScript)