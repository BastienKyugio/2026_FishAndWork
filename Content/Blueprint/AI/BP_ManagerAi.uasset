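; Manager AI character that walks a one-shot patrol route and marks the rooms it touches as scanned.
; BeginPlay scales its walk speed by the FishGameMode coefficient.
; MoveToNextPoint chains AI moves through the patrol points, pauses at the last, returns to the first, then calls the game mode's spawn check and destroys itself.
; Mesh overlaps with a BP_RoomManager trigger RoomIsScanned on that room.
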(event OnComponentBeginOverlap(Mesh)
  (params (OverlappedComponent :type Primitive%20Component%20Object%20Reference) (OtherActor :type Actor%20Object%20Reference) (OtherComp :type Primitive%20Component%20Object%20Reference) (OtherBodyIndex :type Integer) (bFromSweep :type Boolean) (SweepResult :type Hit%20Result%20Structure%20%28by%20ref%29))
  (bind _asbp_room_manager (Utilities|Casting|CastToBP_RoomManager OtherActor))
  (Default|RoomIsScanned _asbp_room_manager))

(event Custom|MoveToNextPoint
  (bind _manager_patrolpoints (Variables|Default|GetManager_PatrolPoints))
  (bind _currentpointindex (Variables|Default|GetCurrentPointIndex))
  (bind _output (Utilities|Array|Get(acopy) _manager_patrolpoints _currentpointindex))
  (Utilities|IsValid _output
    (:Is%20Valid
      (AI|AIMoveTo self (Transformation|GetActorLocation _output) 0 5e+01 false
        (:OnSuccess
          (Development|PrintString "(AI_Manager)  Le Manager a atteint un autre point")
          (if (== (Variables|Default|GetCurrentPointIndex) (Utilities|Array|LastIndex (Variables|Default|GetManager_PatrolPoints)))
            (Utilities|FlowControl|Delay 5.0)
            (AI|AIMoveTo self (Transformation|GetActorLocation (Utilities|Array|Get(acopy) (Variables|Default|GetManager_PatrolPoints))) 0 5e+01 false
              (:OnSuccess
                (Development|PrintString "Fin de pattern")
                (Default|CheckAISpawn (Variables|Default|GetAs%20Fish%20Game%20Mode) 3)
                (Actor|DestroyActor)))
            (else
              (Math|Integer|IncrementInt (Variables|Default|GetCurrentPointIndex)
                (:%20%20
                  (CallFunction|MovetoNextPoint))))))
        (:OnFail
          (Development|PrintString "(AI_Manager) Le Manager n'a pas atteint l'autre point"))))
    (:Is%20Not%20Valid
      (Development|PrintString (Utilities|String|ToString(Integer) (Utilities|Array|Length (Variables|Default|GetManager_PatrolPoints)))))))

(event EventBeginPlay
  (bind _charactermovement (Variables|Character|GetCharacterMovement))
  (bind _asfish_game_mode (Utilities|Casting|CastToFishGameMode (Game|GetGameMode)))
  (bind _output_get (Variables|Default|SetAs%20Fish%20Game%20Mode _asfish_game_mode))
  (Variables|/Script/Engine.CharacterMovementComponent|SetMaxWalkSpeed _charactermovement (* (Variables|/Game/Player/FishGameMode.FishGameMode_C|GetCoef _output_get) (Variables|/Script/Engine.CharacterMovementComponent|GetMaxWalkSpeed _charactermovement))))

(fn ConstructionScript)