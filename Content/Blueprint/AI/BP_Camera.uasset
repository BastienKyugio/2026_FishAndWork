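; BP_Camera is a room-scanning camera that flags its Room as scanned and feeds into the game mode's AI spawning.
; SwitchOn, ScanRoom and SwitchOff form a timeline chain that tilts GEOCamera, sweeps it in yaw, then tilts it back, passing the saved rotation between stages.
; RoomIsScanned fires on the Room before the sweep starts.
; When switch-off finishes, it calls CheckAISpawn on FishGameMode and resets the saved rotation.
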(event Custom|SwitchOn
  (bind _newtrack_0 (Timeline|SwitchOnTimeline PlayFromStart)
    (:Update
      (Transformation|SetRelativeRotation (Variables|Default|GetGEO_Camera) (Math|Rotator|MakeRotator (Math|Float|Lerp 0.0 -4e+01 _newtrack_0) 0.0 0.0) false false))
    (:Finished
      (Variables|Default|SetSwitchOnRotation (Variables|/Script/Engine.SceneComponent|GetRelativeRotation (Variables|Default|GetGEO_Camera)))
      (Default|RoomIsScanned (Variables|Default|GetRoom))
      (Development|PrintString "RoomIsScanned")
      (CallFunction|ScanRoom))))

(event Custom|ScanRoom
  (bind _newtrack_0 (Timeline|ScanTimeline PlayFromStart)
    (:Update
      (Transformation|SetRelativeRotation (Variables|Default|GetGEO_Camera) (Math|Rotator|MakeRotator (.roll (Variables|Default|GetSwitchOnRotation)) 0.0 (+ (.yaw (Variables|Default|GetSwitchOnRotation)) (Math|Float|Lerp -45.0 45.0 _newtrack_0))) false false))
    (:Finished
      (Variables|Default|SetSwitchOnRotation (Variables|/Script/Engine.SceneComponent|GetRelativeRotation (Variables|Default|GetGEO_Camera)))
      (CallFunction|SwitchOff))))

(event Custom|SwitchOff
  (bind _newtrack_0 (Timeline|SwitchOffTimeline PlayFromStart)
    (:Update
      (Transformation|SetRelativeRotation (Variables|Default|GetGEO_Camera) (Math|Rotator|MakeRotator (+ (Math|Float|Lerp 0.0 4e+01 _newtrack_0) (.roll (Variables|Default|GetSwitchOnRotation))) (.pitch (Variables|Default|GetSwitchOnRotation)) (.yaw (Variables|Default|GetSwitchOnRotation))) false false))
    (:Finished
      (Default|CheckAISpawn (Variables|Default|GetAs%20Fish%20Game%20Mode) 2)
      (Variables|Default|SetSwitchOnRotation "0, 0, 0"))))

(event EventBeginPlay
  (bind _asfish_game_mode (Utilities|Casting|CastToFishGameMode (Game|GetGameMode)))
  (Variables|Default|SetAs%20Fish%20Game%20Mode _asfish_game_mode))

(fn ConstructionScript)