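; BP_AI_Director is an AI director that spawns patrolling NPCs and activates a camera through separate events.
; Each spawn event creates a manager with cart, a manager or a computer scientist at the director's location, ignoring collision.
; It then hands the new pawn its role's patrol points from the director's variables and starts it moving to the next point.
; The camera event only switches on a referenced camera.
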(event Custom|SpawnScientistAI
  (bind _returnvalue (AI|SpawnAIFromClass "/Game/Blueprint/AI/BP_ComputerScientist.BP_ComputerScientist_C" 0 (Transformation|GetActorLocation) "0, 0, 0" true 0))
  (bind _asbp_computer_scientist (Utilities|Casting|CastToBP_ComputerScientist _returnvalue))
  (Variables|/Game/Blueprint/AI/BP_ComputerScientist.BP_ComputerScientist_C|SetScientist_PatrolPoints _asbp_computer_scientist (Variables|Default|GetScientist_PointsSpawner))
  (Default|MovetoNextPoint _asbp_computer_scientist))

(event Custom|SpawnManagerWithCart
  (bind _returnvalue (AI|SpawnAIFromClass "/Game/Blueprint/AI/BP_ManagerWithCart.BP_ManagerWithCart_C" 0 (Transformation|GetActorLocation) "0, 0, 0" true 0))
  (bind _asbp_manager_with_cart (Utilities|Casting|CastToBP_ManagerWithCart _returnvalue))
  (Variables|/Game/Blueprint/AI/BP_ManagerWithCart.BP_ManagerWithCart_C|SetCart_PatrolPoints _asbp_manager_with_cart (Variables|Default|GetManagerWithCart_PointSpawner))
  (Default|MovetoNextPoint _asbp_manager_with_cart))

(event Custom|SpawnCamera
  (Default|Switchon (Variables|Default|GetCamera)))

(event Custom|SpawnManagerAI
  (bind _returnvalue (AI|SpawnAIFromClass "/Game/Blueprint/AI/BP_ManagerAi.BP_ManagerAi_C" 0 (Transformation|GetActorLocation) "0, 0, 0" true 0))
  (bind _asbp_manager_ai (Utilities|Casting|CastToBP_ManagerAi _returnvalue))
  (Variables|/Game/Blueprint/AI/BP_ManagerAi.BP_ManagerAi_C|SetManager_PatrolPoints _asbp_manager_ai (Variables|Default|GetManager_PointsSpawner))
  (Default|MovetoNextPoint _asbp_manager_ai))

(fn ConstructionScript)