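; Computer scientist AI character that walks a patrol route through a door, inspects the player's workstation and punishes open pirated software.
; Recursive AIMoveTo steps through the patrol points, opening the door at the second and running the check at the last.
; A catch adds suspicion, logs a cycle stat and plays an angry animation.
; It then returns to the first point, closes the door, notifies the game mode's spawn check and destroys itself.
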(event Custom|MoveToNextPoint
  (bind _scientist_patrolpoints (Variables|Default|GetScientist_PatrolPoints))
  (bind _currentpointindex (Variables|Default|GetCurrentPointIndex))
  (bind _output (Utilities|Array|Get(acopy) _scientist_patrolpoints _currentpointindex))
  (Utilities|IsValid _output
    (:Is%20Valid
      (Default|SetWalkInf (Variables|Default|GetAs%20ABP%20Informaticien))
      (AI|AIMoveTo self (Transformation|GetActorLocation _output) 0 5e+01 false
        (:OnSuccess
          (Development|PrintString "(AI_Scientist)  Le Scientist a atteint un autre point")
          (if (== (Variables|Default|GetCurrentPointIndex) (Utilities|Array|LastIndex (Variables|Default|GetScientist_PatrolPoints)))
            (CallFunction|AnalysePc)
            (Utilities|FlowControl|Delay 5.0)
            (if (Variables|Default|GetCaught)
              (Default|SetAngry (Variables|Default|GetAs%20ABP%20Informaticien))
              (Utilities|FlowControl|Delay 2.0)
              (else
                (Development|PrintString "Hello")))
            (Default|SetWalkInf (Variables|Default|GetAs%20ABP%20Informaticien))
            (AI|AIMoveTo self (Transformation|GetActorLocation (Utilities|Array|Get(acopy) (Variables|Default|GetScientist_PatrolPoints))) 0 5e+01 false
              (:then
                (Utilities|FlowControl|Delay 0.5)
                (Default|CloseDoor (Variables|Default|GetDoor)))
              (:OnSuccess
                (Development|PrintString "Fin de pattern")
                (Default|CheckAISpawn (Variables|Default|GetAs%20Fish%20Game%20Mode) 2)
                (Actor|DestroyActor)))
            (else
              (if (== (Variables|Default|GetCurrentPointIndex) 1)
                (Development|PrintString "Porte")
                (Default|OpenDoor (Variables|Default|GetDoor)))
              (Math|Integer|IncrementInt (Variables|Default|GetCurrentPointIndex)
                (:%20%20
                  (CallFunction|MovetoNextPoint))))))
        (:OnFail
          (Development|PrintString "(AI_Scientist) Le Scientist n'a pas atteint l'autre point"))))
    (:Is%20Not%20Valid
      (Development|PrintString (Utilities|String|ToString(Integer) (Utilities|Array|Length (Variables|Default|GetScientist_PatrolPoints)))))))

(event Custom|AnalysePc
  (bind _as_fish_game_mode (Variables|Default|GetAs%20Fish%20Game%20Mode))
  (bind _cyclestats (Variables|/Game/Player/FishGameMode.FishGameMode_C|GetCycleStats _as_fish_game_mode))
  (Default|SetJump (Variables|Default|GetAs%20ABP%20Informaticien))
  (Development|PrintString "Analyse")
  (bind _returnvalue (Actor|GetActorOfClass "/Game/Blueprint/BP_WorkStation.BP_WorkStation_C"))
  (bind _aswbp_os_main (Utilities|Casting|CastToWBP_OS_Main (UserInterface|GetUserWidgetObject (Variables|/Game/Blueprint/BP_WorkStation.BP_WorkStation_C|GetWidget _returnvalue))))
  (Variables|Default|SetAs%20WBP%20OS%20Main _aswbp_os_main)
  (if (Variables|/Game/UI/PC/WBP_OS_Main.WBP_OS_Main_C|GetPirateSoftware_IsOpen _aswbp_os_main)
    (Variables|Default|SetCaught true)
    (Default|AddSuspicion _as_fish_game_mode 5e+01)
    (Utilities|Struct|SetmembersinS_CycleStats _cyclestats (+ (.Susp_Conspir_UsePiratedSoftware (Utilities|Struct|BreakS_CycleStats _cyclestats)) 1))
    (else
      (Variables|Default|SetCaught false))))

(event EventBeginPlay
  (bind _charactermovement (Variables|Character|GetCharacterMovement))
  (bind _asabp_informaticien (Utilities|Casting|CastToABP_Informaticien (Components|SkeletalMesh|GetAnimInstance (Variables|Character|GetMesh))))
  (Variables|Default|SetAs%20ABP%20Informaticien _asabp_informaticien)
  (bind _asfish_game_mode (Utilities|Casting|CastToFishGameMode (Game|GetGameMode)))
  (bind _output_get (Variables|Default|SetAs%20Fish%20Game%20Mode _asfish_game_mode))
  (Variables|/Script/Engine.CharacterMovementComponent|SetMaxWalkSpeed _charactermovement (* (Variables|/Game/Player/FishGameMode.FishGameMode_C|GetCoef _output_get) (Variables|/Script/Engine.CharacterMovementComponent|GetMaxWalkSpeed _charactermovement))))

(fn ConstructionScript)