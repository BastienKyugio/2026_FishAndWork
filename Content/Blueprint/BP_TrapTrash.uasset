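; BP_TrapTrash is a trash trap that destroys file actors (BP_FIle) overlapping its DestroyBox, after a short delay and a fire sound.
; Files listed in the FishGameMode's TargetTaskFile are removed from it and counted on the tasks UI, and emptying that list triggers ChangeTask.
; Other actors are ignored, and GetItemPickable returns a fixed enum value.
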(event OnComponentBeginOverlap(DestroyBox)
  (params (OverlappedComponent :type Primitive%20Component%20Object%20Reference) (OtherActor :type Actor%20Object%20Reference) (OtherComp :type Primitive%20Component%20Object%20Reference) (OtherBodyIndex :type Integer) (bFromSweep :type Boolean) (SweepResult :type Hit%20Result%20Structure%20%28by%20ref%29))
  (Variables|Default|SetObjectOnTrash OtherActor)
  (bind _asfish_game_mode (Utilities|Casting|CastToFishGameMode (Game|GetGameMode)))
  (bind _asbp_file (Utilities|Casting|CastToBP_FIle (Variables|Default|GetObjectOnTrash)))
  (if (Utilities|Array|ContainsItem (Variables|/Game/Player/FishGameMode.FishGameMode_C|GetTargetTaskFile _asfish_game_mode) _asbp_file)
    (Utilities|Array|RemoveItem (Variables|/Game/Player/FishGameMode.FishGameMode_C|GetTargetTaskFile _asfish_game_mode) _asbp_file)
    (Math|Integer|IncrementInt (Variables|/Game/UI/WBP_Tasks.WBP_Tasks_C|GetAmount (Variables|/Game/Player/FishGameMode.FishGameMode_C|GetTasksUI _asfish_game_mode))
      (:%20%20
        (Default|TaskDestroyFiles (Variables|/Game/Player/FishGameMode.FishGameMode_C|GetTasksUI _asfish_game_mode))
        (if (Utilities|Array|IsEmpty (Variables|/Game/Player/FishGameMode.FishGameMode_C|GetTargetTaskFile _asfish_game_mode))
          (Default|ChangeTask _asfish_game_mode)))))
  (Utilities|FlowControl|Delay 0.2)
  (Audio|PlaySound2D "/Game/Sound_Design/SD_Fire.SD_Fire" 1.0 1.0 0.0 0 0)
  (Actor|DestroyActor (Variables|Default|GetObjectOnTrash)))

(fn ConstructionScript)

(fn GetItemPickable
  (return "NewEnumerator1"))