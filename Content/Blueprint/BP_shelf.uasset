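; Shelf actor with five slots that stores BP_FIle objects the player carries.
; BeginPlay spawns the initial files attached to the slots and runs a Timeline that bobs the slots with sine and cosine offsets.
; PutFileOn snaps the held object into the first empty slot, clears the player's holding state and HUD prompts, and advances the tidy-up task for Cart-tagged items.
; OnInteract has no effect.
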(event Custom|PutFileOn
  (bind _ascharacter_controller (CallFunction|GetPlayerController))
  (bind _as_fish_game_mode (Variables|Default|GetAs%20Fish%20Game%20Mode))
  (bind _tasksui (Variables|/Game/Player/FishGameMode.FishGameMode_C|GetTasksUI _as_fish_game_mode))
  (if (and (Variables|/Game/Player/BP_FirstPersonController.BP_FirstPersonController_C|GetIsHoldingPickableObject (CallFunction|GetPlayerController)) (< (Variables|Default|GetIndexSlotEmpty) (Utilities|Array|Length (Variables|Default|GetSlotsList))))
    (Audio|PlaySound2D "/Game/Sound_Design/MSS_WaterPush.MSS_WaterPush" 0.5 1.0 0.0 0 0)
    (bind (_array_element _array_index) (Utilities|Array|ForEachLoopwithBreak (Variables|Default|GetFiles) :!label _label)
      (:LoopBody
        (Utilities|IsValid _array_element
          (:Is%20Valid
            (Development|PrintString "Plein"))
          (:Is%20Not%20Valid
            (Variables|Default|SetIndexSlotEmpty _array_index)
            (Class|BPIInteract|OnDrop(Message) (Variables|/Game/Player/BP_FirstPersonController.BP_FirstPersonController_C|GetHeldObject (CallFunction|GetPlayerController)))
            (if (Actor|ActorHasTag (Variables|/Game/Player/BP_FirstPersonController.BP_FirstPersonController_C|GetHeldObject (CallFunction|GetPlayerController)) "Cart")
              (Math|Integer|IncrementInt (Variables|/Game/UI/WBP_Tasks.WBP_Tasks_C|GetAmount _tasksui)
                (:%20%20
                  (Default|TaskTidyUpFiles _tasksui)
                  (Utilities|Array|RemoveItem (Variables|/Script/Engine.Actor|GetTags (Variables|/Game/Player/BP_FirstPersonController.BP_FirstPersonController_C|GetHeldObject (CallFunction|GetPlayerController))) "Cart"))))
            (Transformation|DetachFromActor (Variables|/Game/Player/BP_FirstPersonController.BP_FirstPersonController_C|GetHeldObject (CallFunction|GetPlayerController)) "KeepWorld" "KeepWorld" "KeepWorld")
            (Transformation|AttachComponentToComponent (Variables|/Game/Player/BP_FirstPersonController.BP_FirstPersonController_C|GetHeldObject (CallFunction|GetPlayerController)) (Utilities|Array|Get(acopy) (Variables|Default|GetSlotsList) (Variables|Default|GetIndexSlotEmpty)) "None" "SnapToTarget" "SnapToTarget" "SnapToTarget" true)
            (bind _asbp_file (Utilities|Casting|CastToBP_FIle (Variables|/Game/Player/BP_FirstPersonController.BP_FirstPersonController_C|GetHeldObject (CallFunction|GetPlayerController))))
            (Physics|SetSimulatePhysics (Variables|/Game/Blueprint/BP_Interactable_Base.BP_Interactable_Base_C|GetSkeletalMesh _asbp_file) false)
            (Utilities|Array|SetArrayElem (Variables|Default|GetFiles) _array_index _asbp_file)
            (Development|PrintString "(Shelves) L'objet est rané dans l'étagère")
            (Variables|/Game/Player/BP_FirstPersonController.BP_FirstPersonController_C|SetHeldObject _ascharacter_controller 0)
            (Variables|/Game/Player/BP_FirstPersonController.BP_FirstPersonController_C|SetIsHoldingPickableObject _ascharacter_controller false)
            (Variables|/Game/Player/BP_FirstPersonController.BP_FirstPersonController_C|SetCurrentState _ascharacter_controller "NewEnumerator0")
            (Widget|SetVisibility (Variables|/Game/UI/WBP_HUD.WBP_HUD_C|GetTXT_Drop (Variables|/Game/Player/BP_FirstPersonController.BP_FirstPersonController_C|GetHUD (CallFunction|GetPlayerController))) "Hidden")
            (goto _label Break)))))
    (else
      (Development|PrintString "(Shelves) Le joueur n'a pas d'objet en main/ Pas d'emplacement de libre"))))

(event EventBeginPlay
  (bind _asfish_game_mode (Utilities|Casting|CastToFishGameMode (Game|GetGameMode)))
  (Variables|Default|SetAs%20Fish%20Game%20Mode _asfish_game_mode)
  (bind _output_get (Variables|Default|SetSlotsList (Utilities|Array|MakeArray (Variables|Default|GetSlot_01) (Variables|Default|GetSlot_02) (Variables|Default|GetSlot_03) (Variables|Default|GetSlot_04) (Variables|Default|GetSlot_05))))
  (Utilities|Array|Resize (Variables|Default|GetFiles) (Utilities|Array|Length _output_get))
  (for (_array_element _array_index) (Variables|Default|GetInitialFilesToSpawn)
    (bind _returnvalue (Game|SpawnActorfromClass "/Game/Blueprint/BP_FIle.BP_FIle_C" (Transformation|GetRelativeTransform (Utilities|Array|Get(acopy) (Variables|Default|GetSlotsList) _array_index)) "Undefined" "MultiplyWithRoot" 0 _array_element 0))
    (Transformation|AttachComponentToComponent _returnvalue (Utilities|Array|Get(acopy) (Variables|Default|GetSlotsList) _array_index) "None" "SnapToTarget" "SnapToTarget" "SnapToTarget" true)
    (Utilities|Array|SetArrayElem (Variables|Default|GetFiles) _array_index _returnvalue)
    (for _array_element_2 (Variables|Default|GetSlotsList)
      (Utilities|Array|Add (Variables|Default|GetInitialRelativeLocation) (Variables|/Script/Engine.SceneComponent|GetRelativeLocation _array_element_2))
      (bind _newtrack_0 (Timeline|Timeline Play)
        (:Update
          (for (_array_element_3 _array_index_2) (Variables|Default|GetSlotsList)
            (Transformation|SetRelativeLocation _array_element_3 (+ (Utilities|Array|Get(acopy) (Variables|Default|GetInitialRelativeLocation) _array_index_2) (Math|Vector|MakeVector (/ (Math|Trig|Sin(Radians) _newtrack_0) 3.0) (/ (Math|Trig|Cos(Radians) _newtrack_0) 4.0) _newtrack_0)) true true)))))))

(event EventOnInteract
  (Utilities|IsValid (Variables|/Game/Player/BP_FirstPersonController.BP_FirstPersonController_C|GetHeldObject (CallFunction|GetPlayerController))
    (:Is%20Valid
      (for _array_element (Variables|Default|GetSlotsList)
        _))))

(fn ConstructionScript)

(fn GetItemPickable
  (return "NewEnumerator2"))