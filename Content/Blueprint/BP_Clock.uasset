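; BP_Clock is an animated analog clock actor that registers itself with the FishGameMode on BeginPlay.
; A timeline starts right after registration, and its elapsed-hour track rotates both hand components on the pitch axis.
; The big hand makes one continuous turn per hour unit, while the small hand jumps in hour steps from a fixed starting offset.
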(event EventBeginPlay
  (bind _asfish_game_mode (Utilities|Casting|CastToFishGameMode (Game|GetGameMode)))
  (Variables|/Game/Player/FishGameMode.FishGameMode_C|SetClock _asfish_game_mode self)
  (bind _heure_ecoule (Timeline|HorlogeTImeline PlayFromStart)
    (:Update
      (Transformation|SetRelativeRotation (Variables|Default|GetGEO_Clock_Big_Indicator) (Math|Rotator|MakeRotator 0.0 (* _heure_ecoule -3.6e+02) 0.0) false false)
      (Transformation|SetRelativeRotation (Variables|Default|GetGEO_Clock_Small_Indicator) (Math|Rotator|MakeRotator 0.0 (Math|Conversions|ToFloat(Integer) (* (+ (* (Math|Float|Floor _heure_ecoule) 30) 240) -1)) 0.0) false true))))

(fn ConstructionScript)